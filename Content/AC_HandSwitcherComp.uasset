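; Component on the VR character pawn that spawns and removes hand-tracking actors as tracking availability changes.
; After waiting for a controller, it initializes on the locally controlled pawn, then checks left-hand motion controller validity every tick.
; Changes go through SR_SetHandTracked, intended for the server, which destroys current hands and spawns left and right actors only when tracked.
; Spawned hands receive their motion controllers; attachment code is unused.
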(event `self.ReceiveBeginPlay`
  ;[0 1 0.1869] Begin Play
  (bind _asvrcharacter (cast `VRCharacter` (`self.GetOwner`)))
  (bind _output_get (set `self.OwnerPawn` _asvrcharacter))
  (`/Engine/EditorBlueprintResources/StandardMacros.IsValid` (`Pawn.GetController` _output_get) :!label _label
    (:`Is Valid`
      ;[1 1 1] initialisation des mains si on est localement controllé
      (if (`Pawn.IsLocallyControlled` _output_get)
        (`self.HandSwitcher` true)
        (else
          (`BPFL_GenericTools.PI_Print` "pawn is not locally controlled, we dont spawn hands" "" "PI_Debug"))))
    (:`Is Not Valid`
      (`KismetSystemLibrary.Delay` 0.1)
      (goto _label))))

(event `self.ReceiveTick`
  (params (DeltaSeconds :type "Float (single-precision)"))
  (`self.HandSwitcher` false))

(event `SR_SetHandTracked`
  (params (bTracked :type Boolean))
  ;[1 1 1] Hands
  (bind _output_get (set `self.bHandsTracked` bTracked))
  (`self.SpawnHands` _output_get))

(fn `HandSwitcher`
  (params (ForceInitialisation :type Boolean))
  (bind _forceinitialisation (`local.ForceInitialisation`))
  ;[1 1 1] on cherche si les mains sont trackées ou non
  (bind _motioncontrollerdata (`HeadMountedDisplayFunctionLibrary.GetMotionControllerData` (`self.OwnerPawn`) "Left"))
  (bind _bvalid (break `XRMotionControllerData` _motioncontrollerdata))
  ;[1 1 1] Si la valeur change ou qu'on force l'initialisation, alors on informe tout le monde
  (if (or (!= (`self.bHandsTracked`) _bvalid) _forceinitialisation)
    (`self.SR_SetHandTracked` _bvalid)
    (elif _forceinitialisation
      (`self.SR_SetHandTracked` false))))

(fn `OnRep_bHandsTracked`)

(fn `SpawnHands`
  (params (HandsTracked :type Boolean))
  (bind _ownerpawn (`self.OwnerPawn`))
  (bind _currenthandl (`self.CurrentHandL`))
  (bind _currenthandr (`self.CurrentHandR`))
  (bind _ownerpawn_2 (`self.OwnerPawn`))
  ;[1 1 1] Should be called on server
  ;[1 1 1] destruction des ancienens mains
  (`/Engine/EditorBlueprintResources/StandardMacros.IsValid` _currenthandl
    (:`Is Valid`
      (`Actor.K2_DestroyActor` _currenthandl))
    (:`Is Not Valid`
      _))
  (`/Engine/EditorBlueprintResources/StandardMacros.IsValid` _currenthandr
    (:`Is Valid`
      (`Actor.K2_DestroyActor` _currenthandr))
    (:`Is Not Valid`
      _))
  ;[1 1 1] et on fait spawn les bonnes mains
  (`BPFL_GenericTools.PI_Print` "spawn new hands ! hand trackign activated ?" (`KismetStringLibrary.Conv_BoolToString` HandsTracked) "PI_Debug")
  (if HandsTracked
    (bind _returnvalue (`|SpawnActorFromClass` (`self.HandTrackingLeftClass`) (`KismetMathLibrary.MakeTransform` (0.0 0.0 0.0)) "AlwaysSpawn" "SelectDefaultAtRuntime" _ownerpawn_2 (`VRBaseCharacter.LeftMotionController` (`self.OwnerPawn`)) _ownerpawn_2))
    (set `self.CurrentHandL` _returnvalue)
    (bind _returnvalue_2 (`|SpawnActorFromClass` (`self.HandTrackingRightClass`) (`KismetMathLibrary.MakeTransform` (0.0 0.0 0.0)) "AlwaysSpawn" "SelectDefaultAtRuntime" _ownerpawn (`VRBaseCharacter.RightMotionController` (`self.OwnerPawn`)) _ownerpawn))
    (set `self.CurrentHandR` _returnvalue_2)))